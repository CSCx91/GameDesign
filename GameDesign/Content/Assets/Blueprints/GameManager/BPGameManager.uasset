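; Game manager actor that raises a difficulty value as game time passes.
; Each Tick it reads the elapsed game time and increments GameDifficulty once at least ten seconds have passed since the stored TimeBenchmark, then resets the benchmark to the current time.
; Nothing in this Blueprint consumes the difficulty value, and BeginPlay, overlap and construction logic are empty.
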(event EventBeginPlay)

(event Collision|EventActorBeginOverlap
  (params (OtherActor :type Actor%20Object%20Reference)))

(event EventTick
  (params (DeltaSeconds :type Float%20%28single-precision%29))
  (Variables|Default|SetAmountOfSeconds (Utilities|Time|GetGameTimeinSeconds))
  (if (>= (Variables|Default|GetAmountOfSeconds) (+ (Variables|Default|GetTimeBenchmark) 1e+01))
    (Variables|Default|SetGameDifficulty (+ (Variables|Default|GetGameDifficulty) 1.0))
    (Variables|Default|SetTimeBenchmark (Variables|Default|GetAmountOfSeconds))))

(fn ConstructionScript)