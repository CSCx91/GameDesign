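; Chest spawner actor that scatters a random number of chests, one to three, inside its ChestSpawnArea box.
; The construction script calls SpawnChests, which adds a child actor component at a random point in the box for each chest.
; Placement uses unseeded randomness in the box's relative space, so the layout re-rolls whenever the construction script runs.
; The event graph holds only disabled default events.
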(event EventBeginPlay)

(event Collision|EventActorBeginOverlap
  (params (OtherActor :type Actor%20Object%20Reference)))

(event EventTick
  (params (DeltaSeconds :type Float%20%28single-precision%29)))

(fn ConstructionScript
  (switch int 0
    (:Default
      (CallFunction|SpawnChests))))

(fn SpawnChests
  (bind _chestspawnarea (Variables|Default|GetChestSpawnArea))
  (bind _output_get (Variables|Default|SetBoxLimit (Math|Random|RandomInteger 3)))
  (for _index (range _output_get 2)
    (AddComponent|AddChildActorComponent false (Math|Conversions|ToTransform(Vector) (Math|Random|RandomPointinBoundingBox (Variables|/Script/Engine.SceneComponent|GetRelativeLocation _chestspawnarea) (Variables|/Script/Engine.BoxComponent|GetBoxExtent _chestspawnarea))))))