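; BP_Cyborg is the player Blueprint for the cyborg, holding health and a coin count.
; On BeginPlay it creates and adds separate HUD widgets for crosshair, coins, ammo, rocket reload, utility, XP, movement speed, health and fire rate.
; AnyDamage subtracts from Health and only prints a death message at zero or below.
; AddCoins increments the coin count by one, while Tick and overlap events are empty.
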(event EventBeginPlay
  (bind _returnvalue (UserInterface|CreateWidget "/Game/Cyborg/WB_Crosshair.WB_Crosshair_C"))
  (UserInterface|Viewport|AddtoViewport _returnvalue 0)
  (bind _returnvalue_2 (UserInterface|CreateWidget "/Game/Assets/Prefabs/Coins/HUD_Coins.HUD_Coins_C"))
  (UserInterface|Viewport|AddtoViewport _returnvalue_2 0)
  (bind _returnvalue_3 (UserInterface|CreateWidget "/Game/Assets/Blueprints/HUD/WB_PrimaryAmmo.WB_PrimaryAmmo_C"))
  (UserInterface|Viewport|AddtoViewport _returnvalue_3 0)
  (bind _returnvalue_4 (UserInterface|CreateWidget "/Game/Assets/Blueprints/HUD/WB_RocketReload.WB_RocketReload_C"))
  (UserInterface|Viewport|AddtoViewport _returnvalue_4 0)
  (bind _returnvalue_5 (UserInterface|CreateWidget "/Game/Assets/Blueprints/HUD/WB_Utility.WB_Utility_C"))
  (UserInterface|Viewport|AddtoViewport _returnvalue_5 0)
  (bind _returnvalue_6 (UserInterface|CreateWidget "/Game/Assets/Blueprints/HUD/WB_XP.WB_XP_C"))
  (UserInterface|Viewport|AddtoViewport _returnvalue_6 0)
  (bind _returnvalue_7 (UserInterface|CreateWidget "/Game/Assets/Blueprints/HUD/WB_MovementSpeed.WB_MovementSpeed_C"))
  (UserInterface|Viewport|AddtoViewport _returnvalue_7 0)
  (bind _returnvalue_8 (UserInterface|CreateWidget "/Game/Assets/Blueprints/HUD/WB_Health.WB_Health_C"))
  (UserInterface|Viewport|AddtoViewport _returnvalue_8 0)
  (bind _returnvalue_9 (UserInterface|CreateWidget "/Game/Assets/Blueprints/HUD/WB_FireRate.WB_FireRate_C"))
  (UserInterface|Viewport|AddtoViewport _returnvalue_9 0))

(event Collision|EventActorBeginOverlap
  (params (OtherActor :type Actor%20Object%20Reference)))

(event EventTick
  (params (DeltaSeconds :type Float%20%28single-precision%29)))

(event Game|Damage|EventAnyDamage
  (params (Damage :type Float%20%28single-precision%29) (DamageType :type Damage%20Type%20Object%20Reference) (InstigatedBy :type Controller%20Object%20Reference) (DamageCauser :type Actor%20Object%20Reference))
  (bind _output_get (Variables|Default|SetHealth (- (Variables|Default|GetHealth) Damage)))
  (if (<= _output_get 0.0)
    (Development|PrintString "Player is dead")))

(fn ConstructionScript)

(fn AddCoins
  (Variables|Default|SetNumOfCoins (+ (Variables|Default|GetNumOfCoins) 1)))